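; BP_StreetLamp is a street lamp actor in the Town GravityFree area that can be switched on and off.
; LightOn changes state only when the requested value differs, swapping the lamp mesh between lit and unlit versions and toggling the PointLight's visibility.
; An Interaction event flips the lamp by calling LightOn with the opposite of the current state.
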(event `self.ReceiveBeginPlay`)

(event `LightOn`
  (params (LightOn :type Boolean))
  (if (not (== LightOn (`self.IsLightOn`)))
    (bind _output_get (set `self.IsLightOn` LightOn))
    (if _output_get
      (`StaticMeshComponent.SetStaticMesh` (`self.StreetLamp`) "/Game/AdvancedVillagePack/Meshes/SM_StreetLight_LightsOn.SM_StreetLight_LightsOn")
      (`SceneComponent.SetVisibility` (`self.PointLight`) true true)
      (else
        (`StaticMeshComponent.SetStaticMesh` (`self.StreetLamp`) "/Game/AdvancedVillagePack/Meshes/SM_StreetLight.SM_StreetLight")
        (`SceneComponent.SetVisibility` (`self.PointLight`) false true)))))

(event `/Game/Town/Blueprints/BP_Interface_Interaction.Interaction`
  (`self.LightOn` (not (`self.IsLightOn`))))

(fn `UserConstructionScript`)