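; BP_PlanetTownPC, likely the town's player controller, lets the player interact with whatever is in front of the pawn.
; Each tick it traces a short object-type line along the pawn's forward vector and caches a hit implementing BP_Interface_Interaction as TargetActor, clearing it otherwise.
; Pressing the Interaction input sends InteractionMessage to that cached actor.
; The trace debug line and target-name print are left on.
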(event `self.ReceiveTick`
  (params (DeltaSeconds :type "Float (single-precision)"))
  (bind _returnvalue (`GameplayStatics.GetPlayerPawn` 0))
  (bind _returnvalue_2 (`self.K2_GetActorLocation` _returnvalue))
  (bind (_outhit _returnvalue_3) (`KismetSystemLibrary.LineTraceSingleForObjects` _returnvalue_2 (+ _returnvalue_2 (* (`self.GetActorForwardVector` _returnvalue) 300.0)) (`|MakeArray` "ObjectTypeQuery1" "ObjectTypeQuery2" "ObjectTypeQuery3" "ObjectTypeQuery5" :!type "EObjectTypeQuery Enum") false (`|MakeArray` (`GameplayStatics.GetPlayerPawn` 0) null :!type "Actor Object Reference") "ForOneFrame"))
  (if _returnvalue_3
    (bind (_bblockinghit _binitialoverlap _time _distance _location _impactpoint _normal _impactnormal _physmat _hitactor) (`GameplayStatics.BreakHitResult` _outhit))
    (if (`KismetSystemLibrary.DoesImplementInterface` _hitactor "/Game/Town/Blueprints/BP_Interface_Interaction.BP_Interface_Interaction_C")
      (set `self.TargetActor` _hitactor)
      (`KismetSystemLibrary.PrintString` (`KismetSystemLibrary.GetObjectName` _hitactor))
      (else
        (`/Engine/EditorBlueprintResources/StandardMacros.IsValid` (`self.TargetActor`) :!label _label
          (:`Is Valid`
            (set `self.TargetActor` null)))))
    (else
      (goto _label))))

(event `InputAction|Interaction`
  (params (Key :type "Key Structure"))
  (:`Pressed`
    (`/Engine/EditorBlueprintResources/StandardMacros.IsValid` (`self.TargetActor`)
      (:`Is Valid`
        (message `/Game/Town/Blueprints/BP_Interface_Interaction.Interaction` (`self.TargetActor`))))))

(fn `UserConstructionScript`)